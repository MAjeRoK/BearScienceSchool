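; Chapter 4 plot actor: sends the player to the Captain, who assigns the task of building a space antenna to signal for help.
; On BeginPlay it sets the chapter, shows the task widget and places a bear marker on the Captain.
; A one-shot sphere overlap plays timed dialogue lines with voice sounds, branching on whether an antenna is already in BuildingsDone.
; It then starts Chapter 6 if the antenna exists, otherwise Chapter 5.
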(event OnComponentBeginOverlap(Sphere)
  (params (OverlappedComponent :type Primitive%20Component%20Object%20Reference) (OtherActor :type Actor%20Object%20Reference) (OtherComp :type Primitive%20Component%20Object%20Reference) (OtherBodyIndex :type Integer) (bFromSweep :type Boolean) (SweepResult :type Hit%20Result%20Structure%20%28by%20ref%29))
  (bind _asfirst_person_character (Utilities|Casting|CastToFirstPersonCharacter OtherActor))
  (if (not (Variables|Default|GetIsQuestStarted))
    (Variables|Default|SetIsQuestStarted true)
    (Variables|Default|SetCharacterFirstPerson _asfirst_person_character)
    (Utilities|FlowControl|Delay 1.0)
    (Widget|RemovefromParent (Variables|Default|GetTaskWidget))
    (Default|SetBearMarker (Variables|Default|GetCharacterFirstPerson) "Kapitan")
    (bind _returnvalue (UserInterface|CreateWidget "/Game/MainLogic/GamePlot/WBP_QuestField.WBP_QuestField_C"))
    (bind _output_get (Variables|Default|SetDialogs _returnvalue))
    (UserInterface|Viewport|AddtoViewport _output_get 0)
    (Default|PlayFizikSound (Variables|Default|GetCharacterFirstPerson) "Kapitan")
    (Default|ChangeTask (Variables|Default|GetDialogs) "        Капитан: 
Здравствуй, друг!")
    (Utilities|FlowControl|Delay 2.0)
    (Default|PlayFizikSound (Variables|Default|GetCharacterFirstPerson) "Kapitan")
    (Default|ChangeTask (Variables|Default|GetDialogs) "        Капитан: 
У меня для тебя есть очень важное задание!")
    (Utilities|FlowControl|Delay 3.0)
    (bind _array_element (Utilities|Array|ForEachLoopwithBreak (Variables|/Game/FirstPersonBP/Blueprints/FirstPersonCharacter.FirstPersonCharacter_C|GetBuildingsDone (Variables|Default|GetCharacterFirstPerson)) :!label _label)
      (:LoopBody
        (if (== (.building _array_element) "/Game/MainLogic/Building/BP_Antenna.BP_Antenna_C")
          (Variables|Default|SetAntennaBuilt true)
          (goto _label Break)))
      (:Completed
        (if (Variables|Default|GetAntennaBuilt)
          (Default|PlayFizikSound (Variables|Default|GetCharacterFirstPerson) "Kapitan")
          (Default|ChangeTask (Variables|Default|GetDialogs) "        Капитан: 
Но я вижу, что ты и сам догадался построить Космическую антенну, чтобы подать сигнал бедствия")
          (Utilities|FlowControl|Delay 5.0)
          (Default|PlayFizikSound (Variables|Default|GetCharacterFirstPerson) "Kapitan")
          (Default|ChangeTask (Variables|Default|GetDialogs) "        Капитан: 
Хвалю за находчивость!")
          (Utilities|FlowControl|Delay 3.0)
          (Widget|RemovefromParent (Variables|Default|GetDialogs))
          (Default|StartChapter (Variables|Default|GetCharacterFirstPerson) 6)
          (else
            (Default|PlayFizikSound (Variables|Default|GetCharacterFirstPerson) "Kapitan")
            (Default|ChangeTask (Variables|Default|GetDialogs) "        Капитан: 
У нас нет возможности починить корабль своими силами")
            (Utilities|FlowControl|Delay 3.0)
            (Default|PlayFizikSound (Variables|Default|GetCharacterFirstPerson) "Kapitan")
            (Default|ChangeTask (Variables|Default|GetDialogs) "        Капитан: 
Мы должны позвать на помощь")
            (Utilities|FlowControl|Delay 3.0)
            (Default|PlayFizikSound (Variables|Default|GetCharacterFirstPerson) "Kapitan")
            (Default|ChangeTask (Variables|Default|GetDialogs) "        Капитан: 
Для этого нам нужно построить большую Антенну для передачи сигнала бедствия в космос")
            (Utilities|FlowControl|Delay 5.0)
            (Default|PlayFizikSound (Variables|Default|GetCharacterFirstPerson) "Kapitan")
            (Default|ChangeTask (Variables|Default|GetDialogs) "        Капитан: 
Обрати внимание, что для работы Антенны нам необходимо, чтобы производимая энергия была больше потребляемой")
            (Utilities|FlowControl|Delay 4.0)
            (Default|PlayFizikSound (Variables|Default|GetCharacterFirstPerson) "Kapitan")
            (Default|ChangeTask (Variables|Default|GetDialogs) "        Капитан: 
Для увеличения добычи минералов строй больше Буров")
            (Utilities|FlowControl|Delay 3.0)
            (Default|PlayFizikSound (Variables|Default|GetCharacterFirstPerson) "Kapitan")
            (Default|ChangeTask (Variables|Default|GetDialogs) "        Капитан: 
Возведи Антенну, от тебя зависит наша судьба!")
            (Utilities|FlowControl|Delay 3.0)
            (Widget|RemovefromParent (Variables|Default|GetDialogs))
            (Default|StartChapter (Variables|Default|GetCharacterFirstPerson) 5)))))))

(event EventBeginPlay
  (bind _asfirst_person_character (Utilities|Casting|CastToFirstPersonCharacter (Game|GetPlayerCharacter 0)))
  (bind _output_get (Variables|Default|SetCharacterFirstPerson _asfirst_person_character))
  (Variables|/Game/FirstPersonBP/Blueprints/FirstPersonCharacter.FirstPersonCharacter_C|SetChapter _output_get 4)
  (bind _returnvalue (UserInterface|CreateWidget "/Game/MainLogic/GamePlot/WBP_CurrentTask.WBP_CurrentTask_C"))
  (bind _output_get_2 (Variables|Default|SetTaskWidget _returnvalue))
  (UserInterface|Viewport|AddtoViewport _output_get_2 0)
  (Default|SetTextTask (Variables|Default|GetTaskWidget) "Найдите Капитана")
  (Default|SetBearMarker (Variables|Default|GetCharacterFirstPerson) "Kapitan"))

(fn ConstructionScript)
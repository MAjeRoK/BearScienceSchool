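; BP_Chapter5 runs the fifth story chapter, whose task is to build the space antenna.
; On BeginPlay it sets the player character's chapter and shows the task in a WBP_CurrentTask widget.
; It polls the character's BuildingsDone list every second for a BP_Antenna.
; Once found, it stores the antenna's transform on the character, removes the widget and starts chapter 6.
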(event EventBeginPlay
  (bind _asfirst_person_character (Utilities|Casting|CastToFirstPersonCharacter (Game|GetPlayerCharacter 0)))
  (bind _output_get (Variables|Default|SetCharacterFirstPerson _asfirst_person_character))
  (Variables|/Game/FirstPersonBP/Blueprints/FirstPersonCharacter.FirstPersonCharacter_C|SetChapter _output_get 5)
  (bind _returnvalue (UserInterface|CreateWidget "/Game/MainLogic/GamePlot/WBP_CurrentTask.WBP_CurrentTask_C"))
  (bind _output_get_2 (Variables|Default|SetTaskWidget _returnvalue))
  (UserInterface|Viewport|AddtoViewport _output_get_2 0)
  (Default|SetTextTask (Variables|Default|GetTaskWidget) "Постройте Космическую антенну")
  (bind _array_element (Utilities|Array|ForEachLoopwithBreak (Variables|/Game/FirstPersonBP/Blueprints/FirstPersonCharacter.FirstPersonCharacter_C|GetBuildingsDone (Variables|Default|GetCharacterFirstPerson)) :!label _label)
    (:LoopBody
      (if (== (.building _array_element) "/Game/MainLogic/Building/BP_Antenna.BP_Antenna_C")
        (Variables|Default|SetAntennaBuilt true)
        (Variables|/Game/FirstPersonBP/Blueprints/FirstPersonCharacter.FirstPersonCharacter_C|SetAntennaTransform (Variables|Default|GetCharacterFirstPerson) (.buildtransform _array_element))
        (goto _label Break)))
    (:Completed
      (if (Variables|Default|GetAntennaBuilt)
        (Widget|RemovefromParent (Variables|Default|GetTaskWidget))
        (Default|StartChapter (Variables|Default|GetCharacterFirstPerson) 6)
        (else
          (Utilities|FlowControl|Delay 1.0)
          (goto _label))))))

(fn ConstructionScript)
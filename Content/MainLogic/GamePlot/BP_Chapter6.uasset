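; BP_Chapter6 is the story step where the Captain needs enough energy production to power the Antenna, leading into the game's finale.
; On BeginPlay it sets the player's chapter to 6 and shows Captain dialogue in a quest widget.
; If production falls short of consumption, it shows a task widget and re-checks every second through a Delay loop.
; Once satisfied, it advances to chapter 7, swaps the HUD for a thanks screen and calls the finish cutscene.
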(event EventBeginPlay
  (bind _asfirst_person_character (Utilities|Casting|CastToFirstPersonCharacter (Game|GetPlayerCharacter 0)))
  (bind _output_get (Variables|Default|SetCharacterFirstPerson _asfirst_person_character))
  (Variables|/Game/FirstPersonBP/Blueprints/FirstPersonCharacter.FirstPersonCharacter_C|SetChapter _output_get 6)
  (bind _returnvalue (UserInterface|CreateWidget "/Game/MainLogic/GamePlot/WBP_QuestField.WBP_QuestField_C"))
  (bind _output_get_2 (Variables|Default|SetDialogs _returnvalue))
  (UserInterface|Viewport|AddtoViewport _output_get_2 0)
  (if (>= (Variables|/Game/FirstPersonBP/Blueprints/FirstPersonCharacter.FirstPersonCharacter_C|GetEnergyProducing (Variables|Default|GetCharacterFirstPerson)) (Variables|/Game/FirstPersonBP/Blueprints/FirstPersonCharacter.FirstPersonCharacter_C|GetEnergyConsuming (Variables|Default|GetCharacterFirstPerson)))
    _
    (else
      (Default|PlayFizikSound (Variables|Default|GetCharacterFirstPerson) "Kapitan")
      (Default|ChangeTask (Variables|Default|GetDialogs) "        Капитан: 
Не забудь увеличить производсто энергии, чтобы Антенна заработала")
      (Utilities|FlowControl|Delay 3.0)
      (Widget|SetVisibility (Variables|Default|GetDialogs) "Hidden")
      (bind _returnvalue_2 (UserInterface|CreateWidget "/Game/MainLogic/GamePlot/WBP_CurrentTask.WBP_CurrentTask_C"))
      (bind _output_get_3 (Variables|Default|SetTaskWidget _returnvalue_2))
      (UserInterface|Viewport|AddtoViewport _output_get_3 0)
      (Default|SetTextTask (Variables|Default|GetTaskWidget) "Увеличьте производство энергии")
      (if (>= (Variables|/Game/FirstPersonBP/Blueprints/FirstPersonCharacter.FirstPersonCharacter_C|GetEnergyProducing (Variables|Default|GetCharacterFirstPerson)) (Variables|/Game/FirstPersonBP/Blueprints/FirstPersonCharacter.FirstPersonCharacter_C|GetEnergyConsuming (Variables|Default|GetCharacterFirstPerson))) :!label _label
        (Widget|SetVisibility (Variables|Default|GetDialogs) "Visible")
        (Widget|RemovefromParent (Variables|Default|GetTaskWidget))
        (else
          (Utilities|FlowControl|Delay 1.0)
          (goto _label)))))
  (Default|PlayFizikSound (Variables|Default|GetCharacterFirstPerson) "Kapitan")
  (Default|ChangeTask (Variables|Default|GetDialogs) "        Капитан: 
Ура! Мы будем спасены! Спасибо тебе!")
  (Variables|/Game/FirstPersonBP/Blueprints/FirstPersonCharacter.FirstPersonCharacter_C|SetChapter (Variables|Default|GetCharacterFirstPerson) 7)
  (Utilities|FlowControl|Delay 3.0)
  (Widget|RemovefromParent (Variables|Default|GetDialogs))
  (bind _asfirst_person_hud (Utilities|Casting|CastToFirstPersonHUD (HUD|GetHUD (Game|GetPlayerController 0)))
    (:then
      (Widget|SetVisibility (Variables|/Game/FirstPersonBP/Blueprints/FirstPersonHUD.FirstPersonHUD_C|GetPlayerHUD _asfirst_person_hud) "Hidden"))
    (:CastFailed
      _))
  (bind _returnvalue_3 (UserInterface|CreateWidget "/Game/MainLogic/GamePlot/WBPFinalThanks.WBPFinalThanks_C"))
  (UserInterface|Viewport|AddtoViewport _returnvalue_3 0)
  (Utilities|FlowControl|Delay 5.0)
  (Default|CallEDFinishCutSceene (Variables|Default|GetCharacterFirstPerson)))

(fn ConstructionScript)
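; BP_Chapter0 runs the game's intro: a black screen with audio and Russian captions about an asteroid field and crash-landing on an unknown planet.
; BeginPlay locks input to UI and plays IntroCue while TextCaptions updates a quest-field widget on timed delays.
; After the cue's duration, it spawns the spaceship and adds audio components.
; A Delay loop fades out the black screen, restoring game input and calling StartChapter(1) on FirstPersonCharacter.
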(event Custom|TextCaptions
  (Utilities|FlowControl|Delay 2.0)
  (bind _returnvalue (UserInterface|CreateWidget "/Game/MainLogic/GamePlot/WBP_QuestField.WBP_QuestField_C"))
  (Default|ChangeTask _returnvalue "Внимание, команда, мы заходим в поле астероидов! 
Всем приготовиться!")
  (UserInterface|Viewport|AddtoViewport _returnvalue 0)
  (Utilities|FlowControl|Delay 7.0)
  (Default|ChangeTask _returnvalue "Мы падаем! 
Приготовиться к удару о неизвестную планету!")
  (Utilities|FlowControl|Delay 5.0)
  (Widget|RemovefromParent _returnvalue))

(event EventBeginPlay
  (bind _returnvalue (Game|GetPlayerController 0))
  (bind _introcue (Variables|Default|GetIntroCue))
  (bind _returnvalue_2 (UserInterface|CreateWidget "/Game/MainLogic/GamePlot/WBP_BlackScreen.WBP_BlackScreen_C"))
  (UserInterface|Viewport|AddtoViewport _returnvalue_2 0)
  (Input|SetInputModeUIOnly (Game|GetPlayerController 0) 0 "DoNotLock")
  (Utilities|FlowControl|Delay 1.0)
  (CallFunction|TextCaptions)
  (Components|Activation|SetActive _introcue true true)
  (Utilities|FlowControl|Delay (Variables|/Script/Engine.SoundBase|GetDuration (Variables|/Script/Engine.AudioComponent|GetSound _introcue)))
  (Game|SpawnActorfromClass "/Game/MainLogic/SpaceShip.SpaceShip_C" (Variables|Default|GetSpaceShipTransform) "Undefined" 0 0)
  (AddComponent|AddAudioComponent (Game|GetPlayerCharacter 0) false)
  (if (> (Variables|Default|GetWidgetOpacity) 0.0) :!label _label
    (Utilities|FlowControl|Delay 0.1)
    (Appearance|SetColorandOpacity (Variables|/Game/MainLogic/GamePlot/WBP_BlackScreen.WBP_BlackScreen_C|GetBackground _returnvalue_2) (Utilities|Struct|MakeLinearColor 0.0 0.0 0.0 (Variables|Default|GetWidgetOpacity)) :!class /Script/UMG.Image)
    (Variables|Default|SetWidgetOpacity (- (Variables|Default|GetWidgetOpacity) 0.05))
    (goto _label)
    (else
      (Widget|RemovefromParent _returnvalue_2)
      (Input|SetInputModeGameOnly _returnvalue)
      (AddComponent|AddAudioComponent _returnvalue false)
      (bind _asfirst_person_character (Utilities|Casting|CastToFirstPersonCharacter (Game|GetPlayerCharacter 0)))
      (Default|StartChapter _asfirst_person_character 1))))

(event Collision|EventActorBeginOverlap
  (params (OtherActor :type Actor%20Object%20Reference)))

(event EventTick
  (params (DeltaSeconds :type Float%20%28single-precision%29)))

(fn ConstructionScript)
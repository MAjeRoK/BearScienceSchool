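; Chapter 1 plot actor that runs the game's opening sequence when play begins.
; It shows a black screen widget, plays an intro audio cue for its full duration, then spawns the spaceship at a stored transform.
; A delay loop fades the black background out and removes the widget, then prints a Quest1 message and adds an audio component to the player character.
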(event EventBeginPlay
  (bind _introcue (Variables|Default|GetIntroCue))
  (bind _returnvalue (UserInterface|CreateWidget "/Game/MainLogic/GamePlot/WBP_BlackScreen.WBP_BlackScreen_C"))
  (UserInterface|Viewport|AddtoViewport _returnvalue 0)
  (Utilities|FlowControl|Delay 1.0)
  (Components|Activation|SetActive _introcue true true)
  (Utilities|FlowControl|Delay (Variables|/Script/Engine.SoundBase|GetDuration (Variables|/Script/Engine.AudioComponent|GetSound _introcue)))
  (Game|SpawnActorfromClass "/Game/MainLogic/SpaceShip.SpaceShip_C" (Variables|Default|GetSpaceShipTransform) "Undefined" 0 0)
  (if (> (Variables|Default|GetWidgetOpacity) 0.0) :!label _label
    (Utilities|FlowControl|Delay 0.1)
    (Appearance|SetColorandOpacity (Variables|/Game/MainLogic/GamePlot/WBP_BlackScreen.WBP_BlackScreen_C|GetBackground _returnvalue) (Utilities|Struct|MakeLinearColor 0.0 0.0 0.0 (Variables|Default|GetWidgetOpacity)) :!class /Script/UMG.Image)
    (Variables|Default|SetWidgetOpacity (- (Variables|Default|GetWidgetOpacity) 0.05))
    (goto _label)
    (else
      (Widget|RemovefromParent _returnvalue)
      (Development|PrintString "Quest1")
      (AddComponent|AddAudioComponent (Game|GetPlayerCharacter 0) false))))

(event Collision|EventActorBeginOverlap
  (params (OtherActor :type Actor%20Object%20Reference)))

(event EventTick
  (params (DeltaSeconds :type Float%20%28single-precision%29)))

(fn ConstructionScript)
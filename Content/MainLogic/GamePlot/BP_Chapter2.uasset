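; BP_Chapter2 runs the second story chapter: the player finds the Chemist (Himik), learns to mine minerals, then is sent on to chapter 3.
; BeginPlay sets the chapter, objective widget and marker, and the first sphere overlap by the player starts a timed subtitle dialogue with voice sounds.
; A 0.2-second Delay loop updates the remaining mineral count until 20 more are gained, then enables the helmet's mineral display.
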(event OnComponentBeginOverlap(Sphere)
  (params (OverlappedComponent :type Primitive%20Component%20Object%20Reference) (OtherActor :type Actor%20Object%20Reference) (OtherComp :type Primitive%20Component%20Object%20Reference) (OtherBodyIndex :type Integer) (bFromSweep :type Boolean) (SweepResult :type Hit%20Result%20Structure%20%28by%20ref%29))
  (bind _asfirst_person_character (Utilities|Casting|CastToFirstPersonCharacter OtherActor))
  (if (not (Variables|Default|GetIsQuestStarted))
    (Variables|Default|SetIsQuestStarted true)
    (Variables|Default|SetFirstPersonCharacterVar _asfirst_person_character)
    (Utilities|FlowControl|Delay 1.0)
    (Widget|RemovefromParent (Variables|Default|GetTaskWidget))
    (Default|SetBearMarker (Variables|Default|GetFirstPersonCharacterVar) "Himik")
    (bind _returnvalue (UserInterface|CreateWidget "/Game/MainLogic/GamePlot/WBP_QuestField.WBP_QuestField_C"))
    (bind _output_get (Variables|Default|SetDialogs _returnvalue))
    (UserInterface|Viewport|AddtoViewport _output_get 0)
    (Default|PlayFizikSound (Variables|Default|GetFirstPersonCharacterVar) "Himik")
    (Default|ChangeTask (Variables|Default|GetDialogs) "        Химик: 
Ура, ты выжил при падении нашего корабля!")
    (Utilities|FlowControl|Delay 3.0)
    (Default|PlayFizikSound (Variables|Default|GetFirstPersonCharacterVar) "Himik")
    (Default|ChangeTask (Variables|Default|GetDialogs) "        Химик: 
Посмотри, что я нашел!")
    (Utilities|FlowControl|Delay 2.0)
    (Default|PlayFizikSound (Variables|Default|GetFirstPersonCharacterVar) "Himik")
    (Default|ChangeTask (Variables|Default|GetDialogs) "        Химик: 
Это особые минералы")
    (Utilities|FlowControl|Delay 2.0)
    (Default|PlayFizikSound (Variables|Default|GetFirstPersonCharacterVar) "Himik")
    (Default|ChangeTask (Variables|Default|GetDialogs) "        Химик: 
Они уникальны для этой планеты")
    (Utilities|FlowControl|Delay 3.0)
    (if (> (Variables|/Game/FirstPersonBP/Blueprints/FirstPersonCharacter.FirstPersonCharacter_C|GetMineralsCount (Variables|Default|GetFirstPersonCharacterVar)) 0.0)
      (Default|PlayFizikSound (Variables|Default|GetFirstPersonCharacterVar) "Himik")
      (Default|ChangeTask (Variables|Default|GetDialogs) "        Химик: 
Я смотрю, ты их уже добывал! 
Но ничего, попробуй ещё! 
(Используйте ЛКМ)")
      (else
        (Default|PlayFizikSound (Variables|Default|GetFirstPersonCharacterVar) "Himik")
        (Default|ChangeTask (Variables|Default|GetDialogs) "        Химик: 
Ты можешь их добыть, попробуй! 
(Используйте ЛКМ)")))
    (bind _returnvalue_2 (UserInterface|CreateWidget "/Game/MainLogic/GamePlot/WBP_CurrentTask.WBP_CurrentTask_C"))
    (bind _output_get_2 (Variables|Default|SetTaskWidget _returnvalue_2))
    (UserInterface|Viewport|AddtoViewport _output_get_2 0)
    (Variables|Default|SetMineralsGoal (+ (Variables|/Game/FirstPersonBP/Blueprints/FirstPersonCharacter.FirstPersonCharacter_C|GetMineralsCount (Variables|Default|GetFirstPersonCharacterVar)) 2e+01))
    (if (> (- (Variables|Default|GetMineralsGoal) (Variables|/Game/FirstPersonBP/Blueprints/FirstPersonCharacter.FirstPersonCharacter_C|GetMineralsCount (Variables|Default|GetFirstPersonCharacterVar))) 0.0) :!label _label
      (Default|SetTextTask (Variables|Default|GetTaskWidget) (Utilities|Text|ToText(String) (Utilities|String|Append (Utilities|String|ToString(Text) (Utilities|Text|MakeLiteralText "Добудьте ещё ")) (Utilities|String|ToString(Text) (Utilities|Text|ToText(Float) (Math|Float|Clamp(Float) (- (Variables|Default|GetMineralsGoal) (Variables|/Game/FirstPersonBP/Blueprints/FirstPersonCharacter.FirstPersonCharacter_C|GetMineralsCount (Variables|Default|GetFirstPersonCharacterVar))) 0.0 2e+01) "HalfToEven" false true 1 324 0 0)) (Utilities|String|ToString(Text) (Utilities|Text|MakeLiteralText " минералов")))))
      (Utilities|FlowControl|Delay 0.2)
      (goto _label)
      (else
        (Widget|RemovefromParent (Variables|Default|GetTaskWidget))
        (Default|PlayFizikSound (Variables|Default|GetFirstPersonCharacterVar) "Himik")
        (Default|ChangeTask (Variables|Default|GetDialogs) "        Химик: 
Молодец!")
        (Utilities|FlowControl|Delay 2.0)
        (Default|PlayFizikSound (Variables|Default|GetFirstPersonCharacterVar) "Himik")
        (Default|ChangeTask (Variables|Default|GetDialogs) "        Химик: 
Не шевелись, 
я настраиваю твой шлем")
        (Utilities|FlowControl|Delay 3.0)
        (Default|PlayFizikSound (Variables|Default|GetFirstPersonCharacterVar) "Himik")
        (Default|ChangeTask (Variables|Default|GetDialogs) "        Химик: 
Теперь он будет показывать количество твоих минералов в верхнем левом углу")
        (Variables|/Game/FirstPersonBP/Blueprints/FirstPersonCharacter.FirstPersonCharacter_C|SetMineralsStatOn (Variables|Default|GetFirstPersonCharacterVar) true)
        (Utilities|FlowControl|Delay 5.0)
        (Default|PlayFizikSound (Variables|Default|GetFirstPersonCharacterVar) "Himik")
        (Default|ChangeTask (Variables|Default|GetDialogs) "        Химик: 
Хорошо, попробуй найти Инженера. 
Возможно, он подскажет, как использовать минералы")
        (Utilities|FlowControl|Delay 4.0)
        (Widget|RemovefromParent (Variables|Default|GetDialogs))
        (Default|StartChapter (Variables|Default|GetFirstPersonCharacterVar) 3)))))

(event EventBeginPlay
  (bind _asfirst_person_character (Utilities|Casting|CastToFirstPersonCharacter (Game|GetPlayerCharacter 0)))
  (Variables|Default|SetFirstPersonCharacterVar _asfirst_person_character)
  (Variables|/Game/FirstPersonBP/Blueprints/FirstPersonCharacter.FirstPersonCharacter_C|SetChapter _asfirst_person_character 2)
  (bind _returnvalue (UserInterface|CreateWidget "/Game/MainLogic/GamePlot/WBP_CurrentTask.WBP_CurrentTask_C"))
  (Variables|Default|SetTaskWidget _returnvalue)
  (UserInterface|Viewport|AddtoViewport _returnvalue 0)
  (Default|SetTextTask (Variables|Default|GetTaskWidget) "Найдите Химика")
  (Default|SetBearMarker (Variables|Default|GetFirstPersonCharacterVar) "Himik"))

(fn ConstructionScript)
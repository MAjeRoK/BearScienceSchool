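; Chapter 3 story script: the Engineer's tutorial on building and energy.
; On start it shows a find-the-Engineer task and marker; entering the trigger sphere runs a one-time timed dialogue with voice cues.
; Delay-based polling loops wait for the build menu, a new Solar Panel, more minerals and a new Minerals Mine.
; It then enables the helmet energy readout and starts Chapter 4.
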(event OnComponentBeginOverlap(Sphere)
  (params (OverlappedComponent :type Primitive%20Component%20Object%20Reference) (OtherActor :type Actor%20Object%20Reference) (OtherComp :type Primitive%20Component%20Object%20Reference) (OtherBodyIndex :type Integer) (bFromSweep :type Boolean) (SweepResult :type Hit%20Result%20Structure%20%28by%20ref%29))
  (bind _asfirst_person_character (Utilities|Casting|CastToFirstPersonCharacter OtherActor))
  (if (not (Variables|Default|GetIsQuestStarted))
    (Variables|Default|SetIsQuestStarted true)
    (Variables|Default|SetCharacterFirstPerson _asfirst_person_character)
    (Utilities|FlowControl|Delay 1.0)
    (Widget|RemovefromParent (Variables|Default|GetTaskWidget))
    (Default|SetBearMarker (Variables|Default|GetCharacterFirstPerson) "Inginer")
    (bind _returnvalue (UserInterface|CreateWidget "/Game/MainLogic/GamePlot/WBP_QuestField.WBP_QuestField_C"))
    (bind _output_get (Variables|Default|SetDialogs _returnvalue))
    (UserInterface|Viewport|AddtoViewport _output_get 0)
    (Default|PlayFizikSound (Variables|Default|GetCharacterFirstPerson) "Inginer")
    (Default|ChangeTask (Variables|Default|GetDialogs) "        Инженер: 
Привет!")
    (Utilities|FlowControl|Delay 2.0)
    (Default|PlayFizikSound (Variables|Default|GetCharacterFirstPerson) "Inginer")
    (Default|ChangeTask (Variables|Default|GetDialogs) "        Инженер: 
Ого, ты добыл достаточно много минералов!")
    (Utilities|FlowControl|Delay 3.0)
    (Default|PlayFizikSound (Variables|Default|GetCharacterFirstPerson) "Inginer")
    (Default|ChangeTask (Variables|Default|GetDialogs) "        Инженер: 
Давай я научу тебя их использовать")
    (Utilities|FlowControl|Delay 2.0)
    (Default|PlayFizikSound (Variables|Default|GetCharacterFirstPerson) "Inginer")
    (Default|ChangeTask (Variables|Default|GetDialogs) "        Инженер: 
Открой меню строительства 
(Нажмите клавишу Q)")
    (Variables|/Game/FirstPersonBP/Blueprints/FirstPersonCharacter.FirstPersonCharacter_C|SetCheckDone (Variables|Default|GetCharacterFirstPerson) false)
    (Variables|/Game/FirstPersonBP/Blueprints/FirstPersonCharacter.FirstPersonCharacter_C|SetCheckBuild (Variables|Default|GetCharacterFirstPerson) true)
    (Utilities|FlowControl|Delay 2.0)
    (if (Variables|/Game/FirstPersonBP/Blueprints/FirstPersonCharacter.FirstPersonCharacter_C|GetCheckDone (Variables|Default|GetCharacterFirstPerson)) :!label _label
      (Variables|/Game/FirstPersonBP/Blueprints/FirstPersonCharacter.FirstPersonCharacter_C|SetCheckBuild (Variables|Default|GetCharacterFirstPerson) false)
      (Default|PlayFizikSound (Variables|Default|GetCharacterFirstPerson) "Inginer")
      (Default|ChangeTask (Variables|Default|GetDialogs) "        Инженер: 
Теперь построй Солнечную панель. 
15 минералов будет достаточно. 
(Вращайте камеру и используйте ЛКМ)")
      (Variables|Default|SetBuildingsAmount 0)
      (for _array_element (Variables|/Game/FirstPersonBP/Blueprints/FirstPersonCharacter.FirstPersonCharacter_C|GetBuildingsDone (Variables|Default|GetCharacterFirstPerson))
        (if (== (.building _array_element) "/Game/MainLogic/Building/BP_SolarPanel.BP_SolarPanel_C")
          (Math|Integer|IncrementInt (Variables|Default|GetBuildingsAmount))))
      (Variables|Default|SetBuildingsGoal (+ (Variables|Default|GetBuildingsAmount) 1))
      (if (> (Variables|Default|GetBuildingsGoal) (Variables|Default|GetBuildingsAmount)) :!label _label_2
        (Variables|Default|SetBuildingsAmount 0)
        (for _array_element_2 (Variables|/Game/FirstPersonBP/Blueprints/FirstPersonCharacter.FirstPersonCharacter_C|GetBuildingsDone (Variables|Default|GetCharacterFirstPerson))
          (if (== (.building _array_element_2) "/Game/MainLogic/Building/BP_SolarPanel.BP_SolarPanel_C")
            (Math|Integer|IncrementInt (Variables|Default|GetBuildingsAmount))))
        (Utilities|FlowControl|Delay 1.0)
        (goto _label_2)
        (else
          (Default|PlayFizikSound (Variables|Default|GetCharacterFirstPerson) "Inginer")
          (Default|ChangeTask (Variables|Default|GetDialogs) "        Инженер: 
Отлично!")
          (Utilities|FlowControl|Delay 2.0)
          (Default|PlayFizikSound (Variables|Default|GetCharacterFirstPerson) "Inginer")
          (Default|ChangeTask (Variables|Default|GetDialogs) "        Инженер: 
Солнечная панель производит энергию")
          (Utilities|FlowControl|Delay 2.0)
          (Default|PlayFizikSound (Variables|Default|GetCharacterFirstPerson) "Inginer")
          (Default|ChangeTask (Variables|Default|GetDialogs) "        Инженер: 
Добудь еще минералов 
(В режиме строительства добывать минералы нельзя. Не забудь выключить Q)")
          (bind _returnvalue_2 (UserInterface|CreateWidget "/Game/MainLogic/GamePlot/WBP_CurrentTask.WBP_CurrentTask_C"))
          (bind _output_get_2 (Variables|Default|SetTaskWidget _returnvalue_2))
          (UserInterface|Viewport|AddtoViewport _output_get_2 0)
          (Variables|Default|SetMineralsGoal (+ (Variables|/Game/FirstPersonBP/Blueprints/FirstPersonCharacter.FirstPersonCharacter_C|GetMineralsCount (Variables|Default|GetCharacterFirstPerson)) 5e+01))
          (if (> (- (Variables|Default|GetMineralsGoal) (Variables|/Game/FirstPersonBP/Blueprints/FirstPersonCharacter.FirstPersonCharacter_C|GetMineralsCount (Variables|Default|GetCharacterFirstPerson))) 0.0) :!label _label_3
            (Default|SetTextTask (Variables|Default|GetTaskWidget) (Utilities|Text|ToText(String) (Utilities|String|Append (Utilities|String|ToString(Text) (Utilities|Text|MakeLiteralText "Добудьте ещё ")) (Utilities|String|ToString(Text) (Utilities|Text|ToText(Float) (Math|Float|Clamp(Float) (- (Variables|Default|GetMineralsGoal) (Variables|/Game/FirstPersonBP/Blueprints/FirstPersonCharacter.FirstPersonCharacter_C|GetMineralsCount (Variables|Default|GetCharacterFirstPerson))) 0.0 5e+01) "HalfToEven" false true 1 324 0 0)) (Utilities|String|ToString(Text) (Utilities|Text|MakeLiteralText " минералов")))))
            (Utilities|FlowControl|Delay 0.2)
            (goto _label_3)
            (else
              (Widget|RemovefromParent (Variables|Default|GetTaskWidget))
              (Default|PlayFizikSound (Variables|Default|GetCharacterFirstPerson) "Inginer")
              (Default|ChangeTask (Variables|Default|GetDialogs) "        Инженер: 
Построй Минеральный бур 
(Используй колесо мыши, чтобы переключаться между зданиями)")
              (Variables|Default|SetBuildingsAmount 0)
              (for _array_element_3 (Variables|/Game/FirstPersonBP/Blueprints/FirstPersonCharacter.FirstPersonCharacter_C|GetBuildingsDone (Variables|Default|GetCharacterFirstPerson))
                (if (== (.building _array_element_3) "/Game/MainLogic/Building/BP_MineralsMine.BP_MineralsMine_C")
                  (Math|Integer|IncrementInt (Variables|Default|GetBuildingsAmount))))
              (Variables|Default|SetBuildingsGoal (+ (Variables|Default|GetBuildingsAmount) 1))
              (if (> (Variables|Default|GetBuildingsGoal) (Variables|Default|GetBuildingsAmount)) :!label _label_4
                (Variables|Default|SetBuildingsAmount 0)
                (for _array_element_4 (Variables|/Game/FirstPersonBP/Blueprints/FirstPersonCharacter.FirstPersonCharacter_C|GetBuildingsDone (Variables|Default|GetCharacterFirstPerson))
                  (if (== (.building _array_element_4) "/Game/MainLogic/Building/BP_MineralsMine.BP_MineralsMine_C")
                    (Math|Integer|IncrementInt (Variables|Default|GetBuildingsAmount))))
                (Utilities|FlowControl|Delay 1.0)
                (goto _label_4)
                (else
                  (Default|PlayFizikSound (Variables|Default|GetCharacterFirstPerson) "Inginer")
                  (Default|ChangeTask (Variables|Default|GetDialogs) "        Инженер: 
Ты большой молодец!")
                  (Utilities|FlowControl|Delay 2.0)
                  (Default|PlayFizikSound (Variables|Default|GetCharacterFirstPerson) "Inginer")
                  (Default|ChangeTask (Variables|Default|GetDialogs) "        Инженер: 
Бур добывает минералы из земли, тратя на это энергию")
                  (Utilities|FlowControl|Delay 3.0)
                  (Default|PlayFizikSound (Variables|Default|GetCharacterFirstPerson) "Inginer")
                  (Default|ChangeTask (Variables|Default|GetDialogs) "        Инженер: 
Я настроил твой шлем, чтобы ты мог следить за количеством производимой и потребляемой энергии")
                  (Variables|/Game/FirstPersonBP/Blueprints/FirstPersonCharacter.FirstPersonCharacter_C|SetEnergyStatOn (Variables|Default|GetCharacterFirstPerson) true)
                  (Utilities|FlowControl|Delay 5.0)
                  (Default|PlayFizikSound (Variables|Default|GetCharacterFirstPerson) "Inginer")
                  (Default|ChangeTask (Variables|Default|GetDialogs) "        Инженер: 
Если потребляемой энергии будет больше, чем производимой, то эффективность добычи минералов упадет")
                  (Utilities|FlowControl|Delay 5.0)
                  (Default|PlayFizikSound (Variables|Default|GetCharacterFirstPerson) "Inginer")
                  (Default|ChangeTask (Variables|Default|GetDialogs) "        Инженер: 
Для увеличения производства энергии строй больше Солнечных панелей и Медовых реакторов")
                  (Utilities|FlowControl|Delay 5.0)
                  (Default|PlayFizikSound (Variables|Default|GetCharacterFirstPerson) "Inginer")
                  (Default|ChangeTask (Variables|Default|GetDialogs) "        Инженер: 
А сейчас сходи к нашему Капитану, у него есть для тебя важное задание")
                  (Utilities|FlowControl|Delay 4.0)
                  (Widget|RemovefromParent (Variables|Default|GetDialogs))
                  (Default|StartChapter (Variables|Default|GetCharacterFirstPerson) 4)))))))
      (else
        (Utilities|FlowControl|Delay 1.0)
        (goto _label)))))

(event EventBeginPlay
  (bind _asfirst_person_character (Utilities|Casting|CastToFirstPersonCharacter (Game|GetPlayerCharacter 0)))
  (bind _output_get (Variables|Default|SetCharacterFirstPerson _asfirst_person_character))
  (Variables|/Game/FirstPersonBP/Blueprints/FirstPersonCharacter.FirstPersonCharacter_C|SetChapter _output_get 3)
  (bind _returnvalue (UserInterface|CreateWidget "/Game/MainLogic/GamePlot/WBP_CurrentTask.WBP_CurrentTask_C"))
  (bind _output_get_2 (Variables|Default|SetTaskWidget _returnvalue))
  (UserInterface|Viewport|AddtoViewport _output_get_2 0)
  (Default|SetTextTask (Variables|Default|GetTaskWidget) "Найдите Инженера")
  (Default|SetBearMarker (Variables|Default|GetCharacterFirstPerson) "Inginer"))

(fn ConstructionScript)
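; BP_BaseBuilding is a building that either produces energy or consumes it to generate minerals for the player.
; On BeginPlay it adds its energy rate to the FirstPersonCharacter's producing or consuming total, depending on IsProducingEnergy.
; Each Tick, consumers add minerals to that character at a frame-rate-independent rate, scaled by the clamped producing-to-consuming energy ratio, so power shortages slow output.
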(event EventBeginPlay
  (bind _asfirst_person_character (Utilities|Casting|CastToFirstPersonCharacter (Game|GetPlayerCharacter 0)))
  (if (Variables|Default|GetIsProducingEnergy)
    (Variables|/Game/FirstPersonBP/Blueprints/FirstPersonCharacter.FirstPersonCharacter_C|SetEnergyProducing _asfirst_person_character (+ (Math|Conversions|ToFloat(Integer) (Variables|Default|GetEnergyRate)) (Variables|/Game/FirstPersonBP/Blueprints/FirstPersonCharacter.FirstPersonCharacter_C|GetEnergyProducing _asfirst_person_character)))
    (else
      (Variables|/Game/FirstPersonBP/Blueprints/FirstPersonCharacter.FirstPersonCharacter_C|SetEnergyConsuming _asfirst_person_character (+ (Variables|/Game/FirstPersonBP/Blueprints/FirstPersonCharacter.FirstPersonCharacter_C|GetEnergyConsuming _asfirst_person_character) (Math|Conversions|ToFloat(Integer) (Variables|Default|GetEnergyRate)))))))

(event EventTick
  (params (DeltaSeconds :type Float%20%28single-precision%29))
  (if (not (Variables|Default|GetIsProducingEnergy))
    (bind _asfirst_person_character (Utilities|Casting|CastToFirstPersonCharacter (Game|GetPlayerCharacter 0)))
    (Variables|/Game/FirstPersonBP/Blueprints/FirstPersonCharacter.FirstPersonCharacter_C|SetMineralsCount _asfirst_person_character (+ (Variables|/Game/FirstPersonBP/Blueprints/FirstPersonCharacter.FirstPersonCharacter_C|GetMineralsCount _asfirst_person_character) (* (* (Variables|Default|GetMineralsRate) DeltaSeconds) (Math|Float|Clamp(Float) (/ (Variables|/Game/FirstPersonBP/Blueprints/FirstPersonCharacter.FirstPersonCharacter_C|GetEnergyProducing _asfirst_person_character) (Variables|/Game/FirstPersonBP/Blueprints/FirstPersonCharacter.FirstPersonCharacter_C|GetEnergyConsuming _asfirst_person_character))))))))

(fn ConstructionScript)
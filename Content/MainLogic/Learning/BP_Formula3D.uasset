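; BP_Formula3D is an in-world learning prop that shows formula hints from its MathInfo on a notebook's front and back widget components.
; On BeginPlay it hides its root and children, waits a second, fills both widgets, then makes everything visible again.
; A shared RenderFormula event casts each component's widget to WBP_FormulaHints and passes MathInfo to DisplayInfo.
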(event Custom|RenderFormula
  (params (Widget :type Widget%20Component%20Object%20Reference))
  (bind _aswbp_formula_hints (Utilities|Casting|CastToWBP_FormulaHints (UserInterface|GetUserWidgetObject Widget)))
  (Default|DisplayInfo _aswbp_formula_hints (Variables|Default|GetMathInfo)))

(event EventBeginPlay
  (Rendering|SetVisibility (Variables|Default|GetDefaultSceneRoot) false true)
  (Utilities|FlowControl|Delay 1.0)
  (CallFunction|RenderFormula (Variables|Default|GetNoteBook))
  (CallFunction|RenderFormula (Variables|Default|GetNoteBookBack))
  (Rendering|SetVisibility (Variables|Default|GetDefaultSceneRoot) true true))

(fn ConstructionScript)